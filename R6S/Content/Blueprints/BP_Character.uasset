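; Character Blueprint that sets up first- and third-person weapon views for a networked game.
; OnSetupWeapon attaches WeaponActor to R_GunSocket on ArmMesh when locally controlled, otherwise on the body Mesh, and shows only that mesh.
; BeginPlay and Tick are empty.
; Print-only events named for server, client, multicast and damage calls, plus disconnected role and authority checks, remain as unused networking test code.
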(event `self.ReceiveBeginPlay`)

(event `self.ReceiveTick`
  (params (DeltaSeconds :type "Float (single-precision)")))

(event `ServerPrintString`
  (`KismetSystemLibrary.PrintString` "Server RPC" true true (struct :`G` 0.66 :`B` 1.0 :`A` 1.0) 30.0))

(event `ClientPrintString`
  (`KismetSystemLibrary.PrintString` "Client RPC" true true (struct :`G` 0.66 :`B` 1.0 :`A` 1.0) 30.0))

(event `ApplyDamageToMe`
  (`KismetSystemLibrary.PrintString` "Damaged"))

(event `MulticastPrintString`
  (`KismetSystemLibrary.PrintString` (`KismetStringLibrary.Concat_StrStr` (`KismetSystemLibrary.GetDisplayName` self) "Multicast RPC") true true (struct :`G` 0.66 :`B` 1.0 :`A` 1.0) 30.0))

(event `self.OnSetupWeapon`
  (bind _weaponactor (`self.WeaponActor`))
  (bind _mesh (`self.Mesh`))
  (bind _armmesh (`self.ArmMesh`))
  (if (`self.IsLocallyControlled`)
    (`/Engine/EditorBlueprintResources/StandardMacros.IsValid` (`self.WeaponActor`)
      (:`Is Valid`
        (`self.K2_AttachToComponent` _weaponactor (`self.ArmMesh`) "R_GunSocket" "SnapToTarget" "SnapToTarget" "KeepRelative" true))
      (:`Is Not Valid`
        _))
    (`SceneComponent.SetVisibility` _mesh false true)
    (`SceneComponent.SetVisibility` _armmesh true true)
    (else
      (`/Engine/EditorBlueprintResources/StandardMacros.IsValid` (`self.WeaponActor`)
        (:`Is Valid`
          (`self.K2_AttachToComponent` _weaponactor (`self.Mesh`) "R_GunSocket" "SnapToTarget" "SnapToTarget" "KeepRelative" true))
        (:`Is Not Valid`
          _))
      (`SceneComponent.SetVisibility` _mesh true true)
      (`SceneComponent.SetVisibility` _armmesh false true))))

(fn `UserConstructionScript`)