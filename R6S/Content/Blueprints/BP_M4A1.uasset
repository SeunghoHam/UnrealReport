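; M4A1 rifle weapon Blueprint that supplies firing animations and the muzzle position.
; On fire, it plays a shoot montage on its own skeletal mesh, then casts its owner to BP_Character to play matching montages on the body and arm meshes.
; GetMuzzleLocation returns the world-space location of the weapon mesh's MuzzleSocket.
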(event `self.OnFire`
  (`|PlayMontage` (`self.SkeletalMesh`) "/Game/FPS_Assault_Pack/Animations/Rifle/A_Rifle_Shoot01_Montage.A_Rifle_Shoot01_Montage"
    (:`then`
      (bind _asbp_character (cast `/Game/Blueprints/BP_Character` (`self.GetOwner`)))
      (`|PlayMontage` (`Character.Mesh` _asbp_character) "/Game/AnimStarterPack/Fire_Rifle_Hip_Montage.Fire_Rifle_Hip_Montage"
        (:`then`
          (`|PlayMontage` (`/Game/Blueprints/BP_Character.ArmMesh` _asbp_character) "/Game/FPS_Assault_Pack/Animations/Rifle/A_Arms_Rifle_Shoot01_Montage.A_Arms_Rifle_Shoot01_Montage"))))))

(fn `GetMuzzleLocation`
  (returns (ReturnValue :type "Vector Structure"))
  (bind _returnvalue_location (`KismetMathLibrary.BreakTransform` (`SceneComponent.GetSocketTransform` (`self.SkeletalMesh`) "MuzzleSocket" "RTS_World")))
  (return _returnvalue_location))

(fn `UserConstructionScript`)